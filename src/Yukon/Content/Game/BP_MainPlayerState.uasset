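; BP_MainPlayerState tracks the player's shields, fuel, gold, alive status and controllability.
; AnyDamage subtracts from Shields while the player is alive and controllable; at zero or below it clears both flags and prints a death message.
; AddFuel and AddGold events add the given amounts to their totals, with no clamping.
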(event Custom|AddFuel
  (params (FuelAmountToAdd :type Float%20%28single-precision%29))
  (Variables|Default|SetFuel (+ FuelAmountToAdd (Variables|Default|GetFuel))))

(event Custom|AddGold
  (params (Gold%20to%20Add :type Integer))
  (Variables|Default|SetGold (+ Gold%20to%20Add (Variables|Default|GetGold))))

(event EventBeginPlay)

(event EventTick
  (params (DeltaSeconds :type Float%20%28single-precision%29)))

(event Game|Damage|EventAnyDamage
  (params (Damage :type Float%20%28single-precision%29) (DamageType :type Damage%20Type%20Object%20Reference) (InstigatedBy :type Controller%20Object%20Reference) (DamageCauser :type Actor%20Object%20Reference))
  (if (and (Variables|Default|GetIsControllable) (Variables|Default|GetIsAlive))
    (Variables|Default|SetShields (- (Variables|Default|GetShields) Damage))
    (if (<= (Variables|Default|GetShields) 0.0)
      (Variables|Default|SetIsAlive false)
      (Development|PrintString "You died")
      (Variables|Default|SetIsControllable false))))

(fn ConstructionScript)