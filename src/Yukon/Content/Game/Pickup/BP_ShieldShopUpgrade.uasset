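; BP_ShieldShopUpgrade is a shop upgrade display, named for the shield, that changes its floating text while the main character overlaps it.
; BeginPlay caches the first text render's text and color as defaults.
; Overlap begin applies NewText and NewColor, and overlap end restores the defaults.
; Text changes reach both text renders, color changes only the first, and no purchase or upgrade logic is present.
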(event Custom|SetText
  (params (New%20Text :type Text))
  (Rendering|Components|TextRender|SetText (Variables|Default|GetTextRender) New%20Text))

(event Custom|SetColor
  (params (NewColor :type Color%20Structure))
  (Rendering|Components|TextRender|SetTextRenderColor (Variables|Default|GetTextRender) NewColor))

(event EventBeginPlay
  (bind _textrender (Variables|Default|GetTextRender))
  (Variables|Default|SetDefaultText (Variables|/Script/Engine.TextRenderComponent|GetText _textrender))
  (Variables|Default|SetOriginalCOlor (Variables|/Script/Engine.TextRenderComponent|GetTextRenderColor _textrender)))

(event Collision|EventActorBeginOverlap
  (params (OtherActor :type Actor%20Object%20Reference))
  (Utilities|Casting|CastToBP_MainCharacter OtherActor)
  (CallFunction|SetText (Variables|Default|GetNewText))
  (CallFunction|SetColor (Variables|Default|GetNewColor)))

(event EventTick
  (params (DeltaSeconds :type Float%20%28single-precision%29)))

(event Collision|EventActorEndOverlap
  (params (OtherActor :type Actor%20Object%20Reference))
  (Utilities|Casting|CastToBP_MainCharacter OtherActor)
  (CallFunction|SetText (Variables|Default|GetDefaultText))
  (CallFunction|SetColor (Variables|Default|GetOriginalCOlor)))

(fn ConstructionScript)