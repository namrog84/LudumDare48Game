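; BP_BaseEnemy is an enemy character that moves toward a Blackboard goal and shoots at the player.
; Tick, when movement is enabled, adds constant force along each axis toward that goal location.
; A timeline started at BeginPlay fires event-track shots, spawning BP_EnemyBullet from a sphere, aimed at BP_MainCharacter while the player state reports alive.
; HurtEnemy decrements health and destroys the actor at zero.
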(event Custom|StartFire
  (bind _playerchar (Variables|Default|GetPlayerChar))
  (bind _sphere (Variables|Default|GetSphere))
  (bind _returnvalue (Transformation|GetWorldLocation _sphere))
  (Timeline|Timeline_0 Play
    (:NewTrack_1
      (bind _asbp_main_player_state (Utilities|Casting|CastToBP_MainPlayerState (Variables|/Script/Engine.Pawn|GetPlayerState _playerchar)))
      (if (Variables|/Game/Game/BP_MainPlayerState.BP_MainPlayerState_C|GetIsAlive _asbp_main_player_state)
        (Game|SpawnActorfromClass "/Game/Game/Enemy/BP_EnemyBullet.BP_EnemyBullet_C" (Math|Transform|MakeTransform _returnvalue (Math|Rotator|FindLookatRotation _returnvalue (Transformation|GetActorLocation _playerchar))) "AdjustIfPossibleButDontSpawnIfColliding" 0 0) ; Spawn projectile
      ))))

(event Custom|HurtEnemy
  (bind _output_get (Variables|Default|SetEnemyHealth (- (Variables|Default|GetEnemyHealth) 1)))
  (if (<= _output_get 0)
    (Actor|DestroyActor)))

(event EventBeginPlay
  (Variables|Default|SetBB (AI|GetBlackboard (.AsBP%20Base%20Enemy%20Controller (Utilities|Casting|CastToBP_BaseEnemyController (Pawn|GetController)))))
  (bind _returnvalue (Actor|GetActorOfClass "/Game/Game/BP_MainCharacter.BP_MainCharacter_C"))
  (Variables|Default|SetPlayerChar _returnvalue)
  (CallFunction|StartFire))

(event Collision|EventActorBeginOverlap
  (params (OtherActor :type Actor%20Object%20Reference)))

(event EventTick
  (params (DeltaSeconds :type Float%20%28single-precision%29))
  (bind _charactermovement (Variables|Character|GetCharacterMovement))
  (bind _charactermovement_2 (Variables|Character|GetCharacterMovement))
  (bind _force (Variables|Default|GetForce))
  (bind _charactermovement_3 (Variables|Character|GetCharacterMovement))
  (bind _force_2 (Variables|Default|GetForce))
  (bind _force_3 (Variables|Default|GetForce))
  ;[1 1 1] c
  (Utilities|FlowControl|Sequence
    (:then_0
      (if (Variables|Default|GetEnableMovement)
        (Variables|Default|SetGoalLoc (AI|Components|Blackboard|GetValueasVector (Variables|Default|GetBB) (Variables|Default|GetKey%20Name)))
        (if (> (.x (Variables|Default|GetGoalLoc)) (.x (Transformation|GetActorLocation)))
          (Physics|AddForce _charactermovement_2 (Math|Vector|MakeVector _force 0.0 0.0))
          (else
            (Physics|AddForce _charactermovement_2 (Math|Vector|MakeVector (* _force -1.0) 0.0 0.0))))
        (if (> (.y (Variables|Default|GetGoalLoc)) (.y (Transformation|GetActorLocation)))
          (Physics|AddForce _charactermovement_3 (Math|Vector|MakeVector 0.0 _force_2 0.0))
          (else
            (Physics|AddForce _charactermovement_3 (Math|Vector|MakeVector 0.0 (* _force_2 -1.0) 0.0))))
        (if (> (.z (Variables|Default|GetGoalLoc)) (.z (Transformation|GetActorLocation)))
          (Physics|AddForce _charactermovement (Math|Vector|MakeVector 0.0 0.0 _force_3))
          (else
            (Physics|AddForce _charactermovement (Math|Vector|MakeVector 0.0 0.0 (* _force_3 -1.0)))))))))

(fn ConstructionScript)